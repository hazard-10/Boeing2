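; Eye gaze Blueprint that polls eye-tracking data every tick and toggles a gaze dot component.
; The Gazedot and its children are visible only while GetGazeData returns true.
; Each tick it also runs an undrawn Visibility line trace 1000 units along the gaze direction from the gaze origin.
; The trace result is not used, and nothing here repositions the dot.
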(event `self.ReceiveTick`
  (params (DeltaSeconds :type "Float (single-precision)"))
  (bind (_gazeorigin _gazedirection) (break `EyeTrackerGazeData` (`self.Gaze Data`)))
  (bind (_outgazedata _returnvalue) (`EyeTrackerFunctionLibrary.GetGazeData`))
  (set `self.Gaze Data` _outgazedata)
  (`SceneComponent.SetVisibility` (`self.gazedot`) _returnvalue true)
  (`KismetSystemLibrary.LineTraceSingle` _gazeorigin (+ _gazeorigin (* _gazedirection 1000)) "TraceTypeQuery1"))

(fn `UserConstructionScript`)
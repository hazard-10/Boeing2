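; Cube actor that travels along a spline path and pauses when its PawnSensing component sees a pawn, logged as "detect worker".
; On BeginPlay it finds the Control_path actor and starts a timeline, rate-scaled by Timetocomplete, that maps its track to spline distance for world location and rotation.
; Each sighting stops the timeline, and a retriggerable delay resumes it one second after the last detection.
; The G key only prints a debug string.
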(event `self.ReceiveBeginPlay`
  (`self.EnableInput` null)
  (bind _returnvalue (`GameplayStatics.GetActorOfClass` "/Game/controltest/BP/control_path.control_path_C"))
  (set `self.Splineparas` _returnvalue)
  (`self.Moving`))

(event `Key|G`
  (params (Key :type "Key Structure"))
  (:`Pressed`
    (`KismetSystemLibrary.PrintString` "Hello")))

(event `Moving`
  (bind _spline (`/Game/controltest/BP/control_path.Spline` (`self.Splineparas`)))
  (`TimelineComponent.SetPlayRate` (`self.timeline_path`) (/ 1.0 (`self.Timetocomplete`)))
  (bind (_direction _move_track) (`Timeline|timeline_path` :!label _label)
    (:`Update`
      (bind _returnvalue (`KismetMathLibrary.Lerp` 0.0 (`SplineComponent.GetSplineLength` (`/Game/controltest/BP/control_path.Spline` (`self.Splineparas`))) _move_track))
      (`self.K2_SetActorTransform` (`KismetMathLibrary.MakeTransform` (`SplineComponent.GetLocationAtDistanceAlongSpline` _spline _returnvalue "World") (`SplineComponent.GetRotationAtDistanceAlongSpline` _spline _returnvalue "World"))))))

(event `self.PawnSensing.OnSeePawn`
  (params (Pawn :type "Pawn Object Reference"))
  (`KismetSystemLibrary.PrintString` "detect worker")
  (`|ExecutionSequence`
    (:`then_0`
      (goto _label :!via `Stop`))
    (:`then_1`
      (`KismetSystemLibrary.RetriggerableDelay` 1.0)
      (goto _label))))

(fn `UserConstructionScript`)